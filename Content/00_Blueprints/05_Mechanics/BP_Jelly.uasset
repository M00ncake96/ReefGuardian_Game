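; BP_Jelly is a Paper2D sprite actor, a jelly that bobs endlessly up and down from where it starts.
; BeginPlay stores the start position and calls FloatUpAndDown, whose FlipFlop alternates playing and reversing the JellyMovement timeline, retriggered on finish.
; The timeline lerps only Z toward start plus EndPosition.Z.
; DurationOfTravel feeds the play rate directly, and the DoOnce on Update drives nothing.
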(event Custom|FloatUpAndDown
  (bind _startposition (Variables|Default|GetStartPosition))
  (Utilities|FlowControl|FlipFlop
    (:A
      (Components|Timeline|SetPlayRate (Variables|Default|GetJellyMovement) (Variables|Default|GetDurationOfTravel))
      (bind _alpha (Timeline|JellyMovement PlayFromStart)
        (:Update
          (Transformation|SetWorldLocation (Variables|Default|GetPaperSprite) (Math|Vector|MakeVector (.x _startposition) (.y _startposition) (Math|Float|Lerp (.z _startposition) (+ (.z (Variables|Default|GetStartPosition)) (.z (Variables|Default|GetEndPosition))) _alpha)) false false)
          (Utilities|FlowControl|DoOnce false :!label _label))
        (:Finished
          (CallFunction|FloatUpandDown)
          (goto _label Reset))))
    (:B
      (Timeline|JellyMovement ReverseFromEnd))))

(event EventBeginPlay
  (Variables|Default|SetStartPosition (Transformation|GetWorldLocation (Variables|Default|GetPaperSprite)))
  (CallFunction|FloatUpandDown))

(event Collision|EventActorBeginOverlap
  (params (OtherActor :type Actor%20Object%20Reference)))

(event EventTick
  (params (DeltaSeconds :type Float%20%28single-precision%29)))

(fn ConstructionScript)