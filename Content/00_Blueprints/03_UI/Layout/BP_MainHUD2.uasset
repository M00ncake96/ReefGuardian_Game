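; BP_MainHUD2 is the HUD Blueprint that owns the game's layered UI layout and serves as the access point to it.
; On BeginPlay it creates WBP_StandardLayout2 for the owning player with the InitialScreens, stores it and adds it to the viewport.
; Thin wrapper functions forward layer register, unregister, push, pop and clear calls to that layout by layer name.
; RegisterLayer passes only the name on, leaving its LayerWidget input unused.
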(event EventBeginPlay
  (bind _returnvalue (UserInterface|CreateWidget "/Game/00_Blueprints/03_UI/Layout/WBP_StandardLayout2.WBP_StandardLayout2_C" (Game|Player|GetOwningPlayerController) (Variables|Default|GetInitialScreens)))
  (bind _output_get (Variables|Default|SetStandardLayout _returnvalue))
  (UserInterface|Viewport|AddtoViewport _output_get 0))

(fn ConstructionScript)

(fn GetStandardLayout
  (return (Variables|Default|GetStandardLayout)))

(fn RegisterLayer
  (params (LayerName :type Gameplay%20Tag%20Structure) (LayerWidget :type %20Object%20Reference))
  (bind _returnvalue (Default|RegisterLayer (CallFunction|GetStandardLayout) LayerName))
  (return _returnvalue))

(fn UnRegisterLayer
  (params (LayerName :type Gameplay%20Tag%20Structure))
  (bind _returnvalue (Default|UnRegisterLayer (CallFunction|GetStandardLayout) LayerName))
  (return _returnvalue))

(fn PushContenttoLayer
  (params (LayerName :type Gameplay%20Tag%20Structure :default "(TagName=\"UI.Layer\")") (WidgetClass :type User%20Widget%20Soft%20Class%20Reference))
  (bind _widget (Default|PushContenttoLayer (CallFunction|GetStandardLayout) LayerName WidgetClass))
  (return _widget))

(fn PopContentfromLayer
  (params (LayerName :type Gameplay%20Tag%20Structure))
  (Default|PopContentfromLayer (CallFunction|GetStandardLayout) LayerName)
  (return))

(fn ClearAllLayers
  (Default|ClearAllLayers (CallFunction|GetStandardLayout)))

(fn ClearAllLayersExcept
  (params (ExceptionLayerName :type Gameplay%20Tag%20Structure :default "(TagName=\"UI.Layer\")"))
  (Default|ClearAllLayersExcept (CallFunction|GetStandardLayout) ExceptionLayerName))

(fn ClearLayer
  (params (LayerName :type Gameplay%20Tag%20Structure))
  (Default|ClearLayer (CallFunction|GetStandardLayout) LayerName)
  (return))