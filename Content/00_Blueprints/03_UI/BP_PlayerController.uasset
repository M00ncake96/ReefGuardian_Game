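; Player controller that switches input focus between gameplay and UI, with cursor visibility and game pause handled alongside.
; BeginPlay caches the BP_MainHUD2 reference.
; FocusGame restores game-only input and unpauses, while FocusModal focuses a widget in UI-only or game-and-UI mode with optional pause.
; An unconnected pause toggle would push or pop WBP_PauseMenu on the HUD's menu layer outside the main menu level.
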(event EventBeginPlay
  (bind _asbp_main_hud2 (Utilities|Casting|CastToBP_MainHUD2 (HUD|GetHUD)))
  (Variables|Default|SetRef%20Main%20HUD _asbp_main_hud2))

(event EventTick
  (params (DeltaSeconds :type Float%20%28single-precision%29)))

(fn ConstructionScript)

(fn FocusGame
  (Variables|Default|SetbShowMouseCursor false)
  (Input|SetInputModeGameOnly self true)
  (Class|WidgetBlueprintLibrary|SetFocustoGameViewport)
  (Game|SetGamePaused false))

(fn FocusModal
  (params (WidgetToFocus :type Widget%20Object%20Reference) (Show%20Mouse%20Cursor :type Boolean) (bPaused :type Boolean) (UIOnlyInput? :type Boolean))
  (Variables|Default|SetbShowMouseCursor Show%20Mouse%20Cursor)
  (Game|SetGamePaused bPaused)
  (if UIOnlyInput?
    (Input|SetInputModeUIOnly self WidgetToFocus "DoNotLock" true)
    (else
      (Input|SetInputModeGameandUI self WidgetToFocus "DoNotLock" false true))))