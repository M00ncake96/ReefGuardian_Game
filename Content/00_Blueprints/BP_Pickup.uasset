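; BP_Pickup is a bottle pickup actor that adds itself to the player's inventory on touch.
; Its flipbook starts stopped on the first frame.
; When the player character overlaps the collision component, it sends an add-bottle message to that character, then plays the flipbook as feedback and destroys itself after a short delay.
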(event OnComponentBeginOverlap(Pickup_Collision)
  (params (OverlappedComponent :type Primitive%20Component%20Object%20Reference) (OtherActor :type Actor%20Object%20Reference) (OtherComp :type Primitive%20Component%20Object%20Reference) (OtherBodyIndex :type Integer) (bFromSweep :type Boolean) (SweepResult :type Hit%20Result%20Structure%20%28by%20ref%29))
  (bind _returnvalue (Game|GetPlayerCharacter 0))
  (if (== OtherActor _returnvalue)
    (Class|BPIGameplayHILL|AddBottletoInventory(Message) _returnvalue)
    (CallFunction|PlayFeedback)))

(event Custom|Play_Feedback
  (Components|Timeline|PlayfromStart (Variables|Default|GetPaperFlipbook))
  (Utilities|FlowControl|Delay 0.2)
  (Actor|DestroyActor))

(event EventBeginPlay
  (Audio|Components|Audio|Stop (Variables|Default|GetPaperFlipbook))
  (Class|PaperFlipbookComponent|SetPlaybackPositioninFrames (Variables|Default|GetPaperFlipbook) 0 false))

(event Collision|EventActorBeginOverlap
  (params (OtherActor :type Actor%20Object%20Reference)))

(event EventTick
  (params (DeltaSeconds :type Float%20%28single-precision%29)))

(fn ConstructionScript)