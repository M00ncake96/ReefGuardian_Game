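; BP_JellyTrail is an actor that slides a flash sprite between two spline points when play begins.
; BeginPlay caches the local-space positions of the point at PointIndex and of point 1, then plays the MoveSprite timeline.
; Each update lerps X and Z by the timeline alpha and applies those local values as the sprite's world location.
; It covers a single segment, with no logic to advance along further points.
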(event EventBeginPlay
  (bind _spline (Variables|Default|GetSpline))
  (Variables|Default|SetPoint%20Index (Variables|Default|GetPoint%20Index))
  (Variables|Default|SetCurrentPointPos (Spline|GetLocationatSplinePoint _spline (Variables|Default|GetPoint%20Index) "Local"))
  (Variables|Default|SetTargetPointPos (Spline|GetLocationatSplinePoint _spline 1 "Local"))
  (bind _alpha (Timeline|MoveSprite PlayFromStart)
    (:Update
      (Transformation|SetWorldLocation (Variables|Default|GetBlockFlash_Sprite_2) (Math|Vector|MakeVector (Math|Float|Lerp (.x (Variables|Default|GetCurrentPointPos)) (.x (Variables|Default|GetTargetPointPos)) _alpha) 0.0 (Math|Float|Lerp (.z (Variables|Default|GetCurrentPointPos)) (.z (Variables|Default|GetTargetPointPos)) _alpha)) false false))))

(fn ConstructionScript)